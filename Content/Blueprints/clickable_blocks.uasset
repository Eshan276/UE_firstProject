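; Clickable cube actor that swaps its material and takes 5 Health from the player's my_char.
; BeginPlay enables click events, and a FlipFlop on cube clicks alternates between calling CBFunction and applying the AdvancedFlag material.
; CBFunction holds a second FlipFlop: one branch applies AliasReference, prints and sets the reduced Health, the other applies AdvancedFlag.
; An unconnected copy of the damage logic remains in the EventGraph.
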(event OnClicked(Cube)
  (params (TouchedComponent :type Primitive%20Component%20Object%20Reference) (ButtonPressed :type Key%20Structure))
  (Utilities|FlowControl|FlipFlop
    (:A
      (CallFunction|CBFunction))
    (:B
      (Rendering|Material|SetMaterial (Variables|Default|GetCube) 0 "/Engine/MaterialTemplates/VertexAnimation/AdvancedFlag.AdvancedFlag"))))

(event EventBeginPlay
  (Variables|/Script/Engine.PlayerController|SetbEnableClickEvents (Game|GetPlayerController 0) true))

(event Collision|EventActorBeginOverlap
  (params (OtherActor :type Actor%20Object%20Reference)))

(event EventTick
  (params (DeltaSeconds :type Float%20%28single-precision%29)))

(fn ConstructionScript)

(fn CBFunction
  (bind _returnvalue (Game|GetPlayerCharacter 0))
  (bind _cube (Variables|Default|GetCube))
  (Utilities|FlowControl|FlipFlop
    (:A
      (Rendering|Material|SetMaterial _cube 0 "/DatasmithContent/Materials/AliasReference.AliasReference")
      (bind _asmy_char (Utilities|Casting|CastTomy_char _returnvalue))
      (Development|PrintString (Utilities|String|ToString(Integer) (- (Variables|/Game/Blueprints/my_char.my_char_C|Gethealth _asmy_char) 5)))
      (bind _asmy_char_2 (Utilities|Casting|CastTomy_char _returnvalue))
      (Variables|/Game/Blueprints/my_char.my_char_C|Sethealth _asmy_char_2 (- (Variables|/Game/Blueprints/my_char.my_char_C|Gethealth _asmy_char) 5)))
    (:B
      (Rendering|Material|SetMaterial _cube 0 "/Engine/MaterialTemplates/VertexAnimation/AdvancedFlag.AdvancedFlag"))))