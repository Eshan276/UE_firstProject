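; A crack actor that repairs itself while something overlaps its Box trigger and destroys itself once fully repaired.
; Overlap shows the Widget component and starts a retriggerable-delay loop that repeatedly calls Repair to raise Health, printing each new value.
; Ending the overlap hides the widget and clears the flag that keeps the loop running.
; The trigger does not filter which actor overlaps it.
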(event OnComponentBeginOverlap(Box)
  (params (OverlappedComponent :type Primitive%20Component%20Object%20Reference) (OtherActor :type Actor%20Object%20Reference) (OtherComp :type Primitive%20Component%20Object%20Reference) (OtherBodyIndex :type Integer) (bFromSweep :type Boolean) (SweepResult :type Hit%20Result%20Structure%20%28by%20ref%29))
  (Rendering|SetVisibility (Variables|Default|GetWidget) true false)
  (bind _output_get (Variables|Default|Setisoverlapping true))
  (if _output_get :!label _label
    (if (>= (Variables|Default|Gethealth) 100)
      (Actor|DestroyActor)
      (else
        (CallFunction|Repair)
        (Utilities|FlowControl|RetriggerableDelay 0.2)
        (goto _label)))))

(event OnComponentEndOverlap(Box)
  (params (OverlappedComponent :type Primitive%20Component%20Object%20Reference) (OtherActor :type Actor%20Object%20Reference) (OtherComp :type Primitive%20Component%20Object%20Reference) (OtherBodyIndex :type Integer))
  (Rendering|SetVisibility (Variables|Default|GetWidget) false false)
  (Variables|Default|Setisoverlapping false))

(event Custom|repair
  (bind _output_get (Variables|Default|Sethealth (+ (Variables|Default|Gethealth) 5)))
  (Development|PrintString (Utilities|String|ToString(Integer) _output_get)))

(event EventBeginPlay
  (Rendering|SetVisibility (Variables|Default|GetWidget) false false))

(event Collision|EventActorBeginOverlap
  (params (OtherActor :type Actor%20Object%20Reference)))

(event EventTick
  (params (DeltaSeconds :type Float%20%28single-precision%29)))

(fn ConstructionScript)