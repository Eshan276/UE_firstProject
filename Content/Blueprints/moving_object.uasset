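; Moving-object actor that makes its Sphere component chase the first player character.
; Every Tick it calls MoveComponentTo with a one-second duration, feeding the character's world location and rotation into the relative-space targets, and prints a debug string.
; BeginPlay, overlap and construction logic are empty, and alternative mesh and nav-agent position getters are left unconnected.
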(event EventBeginPlay)

(event Collision|EventActorBeginOverlap
  (params (OtherActor :type Actor%20Object%20Reference)))

(event EventTick
  (params (DeltaSeconds :type Float%20%28single-precision%29))
  (bind _returnvalue (Game|GetPlayerCharacter 0))
  (Components|MoveComponentTo (Variables|Default|GetSphere) (Transformation|GetActorLocation _returnvalue) (Transformation|GetActorRotation _returnvalue) false false 1.0 false)
  (Development|PrintString "letsgo"))

(fn ConstructionScript)